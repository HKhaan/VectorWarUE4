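; BP_VectorWarBullet is the visual actor for one bullet in the VectorWar game state, selected by its bullet index.
; On begin play it gives its sphere a red dynamic instance of the ship material.
; Each tick it copies that bullet's transform and enabled state from the game state to the root's transform and visibility, teleporting the move when the root was hidden.
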(event `self.ReceiveBeginPlay`
  (bind _returnvalue (`PrimitiveComponent.CreateDynamicMaterialInstance` (`self.Sphere`) 0 "/Game/Materials/M_ShipMaterial.M_ShipMaterial" "None"))
  (`MaterialInstanceDynamic.SetVectorParameterValue` _returnvalue "Color" (make `LinearColor` 1.0 0.0 0.0 1.0)))

(event `self.ReceiveTick`
  (params (DeltaSeconds :type "Float (single-precision)"))
  (bind _bulletindex (`self.BulletIndex`))
  (bind _asvwgame_state_base (cast `VWGameStateBase` (`GameplayStatics.GetGameState`)))
  (`SceneComponent.K2_SetWorldTransform` (`self.Root`) (`GameStateInterface.BulletTransform` _asvwgame_state_base _bulletindex) false (not (`SceneComponent.IsVisible` (`self.Root`))))
  (`SceneComponent.SetVisibility` (`self.Root`) (`GameStateInterface.BulletEnabled` _asvwgame_state_base _bulletindex) true))

(fn `UserConstructionScript`)